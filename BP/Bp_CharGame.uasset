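; Player character Blueprint that drives walking, strafing, yaw rotation, sprinting and crouching through Enhanced Input, adding its mapping context on BeginPlay.
; Movement inputs also store their values in animation-facing variables.
; Sprint and crouch change MaxWalkSpeed and update state flags through setters, but releasing crouch sets speed to zero.
; Crouching clears the sprint flag, while the reverse branch is disabled by a false condition.
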(event Input|EnhancedActionEvents|EnhancedInputActionia_Forward
  (params (ActionValue :type Float%20%28double-precision%29) (ElapsedSeconds :type Float%20%28double-precision%29) (TriggeredSeconds :type Float%20%28double-precision%29) (InputAction :type Input%20Action%20Object%20Reference :default "/Game/INPUT/ia_Forward.ia_Forward"))
  (:Triggered
    (Variables|Default|SetspeedFwdAnime2 ActionValue :!label _label)
    (Pawn|Input|AddMovementInput (Transformation|GetActorForwardVector) ActionValue false))
  (:Completed
    (goto _label)))

(event Input|EnhancedActionEvents|EnhancedInputActionia_Right
  (params (ActionValue :type Float%20%28double-precision%29) (ElapsedSeconds :type Float%20%28double-precision%29) (TriggeredSeconds :type Float%20%28double-precision%29) (InputAction :type Input%20Action%20Object%20Reference :default "/Game/INPUT/ia_Right.ia_Right"))
  (:Triggered
    (Variables|Default|SetspeedRgtAnime2 ActionValue :!label _label)
    (Pawn|Input|AddMovementInput (Transformation|GetActorRightVector) ActionValue false))
  (:Completed
    (goto _label)))

(event Input|EnhancedActionEvents|EnhancedInputActionia_Rotate
  (params (ActionValue :type Float%20%28double-precision%29) (ElapsedSeconds :type Float%20%28double-precision%29) (TriggeredSeconds :type Float%20%28double-precision%29) (InputAction :type Input%20Action%20Object%20Reference :default "/Game/INPUT/ia_Rotate.ia_Rotate"))
  (:Triggered
    (Variables|Default|SetspeedYawanime2 ActionValue :!label _label)
    (Pawn|Input|AddControllerYawInput ActionValue))
  (:Completed
    (goto _label)))

(event Input|EnhancedActionEvents|EnhancedInputActionia_Sprint
  (params (ActionValue :type Boolean) (ElapsedSeconds :type Float%20%28double-precision%29) (TriggeredSeconds :type Float%20%28double-precision%29) (InputAction :type Input%20Action%20Object%20Reference :default "/Game/INPUT/ia_Sprint.ia_Sprint"))
  (bind _charactermovement (Variables|Character|GetCharacterMovement))
  (:Triggered
    (Variables|/Script/Engine.CharacterMovementComponent|SetMaxWalkSpeed _charactermovement (Variables|Default|GetspeedSprint))
    (CallFunction|SetIsSprinting ActionValue :!label _label))
  (:Completed
    (Variables|/Script/Engine.CharacterMovementComponent|SetMaxWalkSpeed _charactermovement (Variables|Default|GetspeedValueBase))
    (goto _label)))

(event Input|EnhancedActionEvents|EnhancedInputActionia_crouch
  (params (ActionValue :type Boolean) (ElapsedSeconds :type Float%20%28double-precision%29) (TriggeredSeconds :type Float%20%28double-precision%29) (InputAction :type Input%20Action%20Object%20Reference :default "/Game/INPUT/ia_crouch.ia_crouch"))
  (bind _charactermovement (Variables|Character|GetCharacterMovement))
  (:Triggered
    (Variables|/Script/Engine.CharacterMovementComponent|SetMaxWalkSpeed _charactermovement (Variables|Default|GetspeedCrouch))
    (CallFunction|SetIsCrouching ActionValue :!label _label))
  (:Completed
    (Variables|/Script/Engine.CharacterMovementComponent|SetMaxWalkSpeed _charactermovement 0.0)
    (goto _label)))

(event EventBeginPlay
  (Input|AddMappingContext (PlayerController|LocalPlayerSubsystems|GetEnhancedInputLocalPlayerSubsystem (Game|GetPlayerController 0)) (Variables|Default|GetMapping%20Context) 0 "(bIgnoreAllPressedKeysUntilRelease=True,bForceImmediately=False)"))

(event Collision|EventActorBeginOverlap
  (params (OtherActor :type Actor%20Object%20Reference)))

(event EventTick
  (params (DeltaSeconds :type Float%20%28single-precision%29)))

(fn ConstructionScript)

(fn SetIsSprinting
  (params (bool :type Boolean))
  (bind _output_get (Variables|Default|SetIs%20Sprinting bool))
  (Variables|Default|Setanimesprint _output_get)
  (if (and false (Variables|Default|GetisCrouching))
    (CallFunction|SetIsCrouching false)))

(fn SetIsCrouching
  (params (value :type Boolean))
  (bind _output_get (Variables|Default|SetisCrouching value))
  (Variables|Default|Setanimcrouch _output_get)
  (if (and _output_get (Variables|Default|GetisCrouching))
    (CallFunction|SetIsSprinting false)))