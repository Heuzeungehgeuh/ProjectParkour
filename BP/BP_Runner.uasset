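; BP_Runner is a player character that collects randomly spawned items by running near them, printing "gagné" when its counter hits zero.
; Enhanced Input drives movement, yaw, sprint and crouch speeds.
; A BeginPlay timeline spawns items on each update into AllItem and attempts a distance-based swap sort.
; Tick recolors items within MinDistance, removes BP_JalonChild ones, and draws input-state shapes and lines to items for debugging.
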(event Input|EnhancedActionEvents|EnhancedInputActionia_Forward
  (params (ActionValue :type Float%20%28double-precision%29) (ElapsedSeconds :type Float%20%28double-precision%29) (TriggeredSeconds :type Float%20%28double-precision%29) (InputAction :type Input%20Action%20Object%20Reference :default "/Game/INPUT/ia_Forward.ia_Forward"))
  (:Triggered
    (Pawn|Input|AddMovementInput (Transformation|GetActorForwardVector) ActionValue false)
    (Variables|Debug|Bool|Setforback true))
  (:Completed
    (Variables|Debug|Bool|Setforback false)))

(event Input|EnhancedActionEvents|EnhancedInputActionia_Right
  (params (ActionValue :type Float%20%28double-precision%29) (ElapsedSeconds :type Float%20%28double-precision%29) (TriggeredSeconds :type Float%20%28double-precision%29) (InputAction :type Input%20Action%20Object%20Reference :default "/Game/INPUT/ia_Right.ia_Right"))
  (:Triggered
    (Pawn|Input|AddMovementInput (Transformation|GetActorRightVector) ActionValue false)
    (Variables|Debug|Bool|Setrightleft true))
  (:Completed
    (Variables|Debug|Bool|Setrightleft false)))

(event Input|EnhancedActionEvents|EnhancedInputActionia_Rotate
  (params (ActionValue :type Float%20%28double-precision%29) (ElapsedSeconds :type Float%20%28double-precision%29) (TriggeredSeconds :type Float%20%28double-precision%29) (InputAction :type Input%20Action%20Object%20Reference :default "/Game/INPUT/ia_Rotate.ia_Rotate"))
  (:Triggered
    (Pawn|Input|AddControllerYawInput ActionValue)
    (Variables|Debug|Bool|SetyawTF true))
  (:Completed
    (Variables|Debug|Bool|SetyawTF false)))

(event Input|EnhancedActionEvents|EnhancedInputActionia_Sprint
  (params (ActionValue :type Boolean) (ElapsedSeconds :type Float%20%28double-precision%29) (TriggeredSeconds :type Float%20%28double-precision%29) (InputAction :type Input%20Action%20Object%20Reference :default "/Game/INPUT/ia_Sprint.ia_Sprint"))
  (bind _charactermovement (Variables|Character|GetCharacterMovement))
  (:Triggered
    (Variables|Debug|Bool|Setsprintornot true)
    (Variables|/Script/Engine.CharacterMovementComponent|SetMaxWalkSpeed _charactermovement (Variables|SpeedMovement|GetsprintSpeedMax)))
  (:Completed
    (Variables|Debug|Bool|Setsprintornot false)
    (Variables|/Script/Engine.CharacterMovementComponent|SetMaxWalkSpeed _charactermovement (Variables|SpeedMovement|Getspeedvaluebase))))

(event Input|EnhancedActionEvents|EnhancedInputActionia_crouch
  (params (ActionValue :type Boolean) (ElapsedSeconds :type Float%20%28double-precision%29) (TriggeredSeconds :type Float%20%28double-precision%29) (InputAction :type Input%20Action%20Object%20Reference :default "/Game/INPUT/ia_crouch.ia_crouch"))
  (bind _charactermovement (Variables|Character|GetCharacterMovement))
  (:Started
    (if true
      (Development|PrintString "Crouch On")
      (if true
        (Variables|/Script/Engine.CharacterMovementComponent|SetMaxWalkSpeed _charactermovement (Variables|SpeedMovement|GetcrouchSpeedMin)))))
  (:Completed
    (Variables|/Script/Engine.CharacterMovementComponent|SetMaxWalkSpeed _charactermovement (Variables|SpeedMovement|Getspeedvaluebase))))

(event Input|EnhancedActionEvents|EnhancedInputActionia_Entre
  (params (ActionValue :type Boolean) (ElapsedSeconds :type Float%20%28double-precision%29) (TriggeredSeconds :type Float%20%28double-precision%29) (InputAction :type Input%20Action%20Object%20Reference :default "/Game/INPUT/ia_Entre.ia_Entre")))

(event EventBeginPlay
  (bind _returnvalue (Transformation|GetActorLocation))
  (Input|AddMappingContext (PlayerController|LocalPlayerSubsystems|GetEnhancedInputLocalPlayerSubsystem (Game|GetPlayerController 0)) (Variables|Default|GetMapping%20Context) 0 "(bIgnoreAllPressedKeysUntilRelease=True,bForceImmediately=False)")
  (bind _outactors (Actor|GetAllActorsOfClass (Variables|Default|Gettypetofind)))
  (Variables|Default|SetallItem _outactors)
  (bind _alpha (Timeline|Timeline Play)
    (:Update
      (CallFunction|Spawn _alpha)
      (CallFunction|NumbertoStart)
      (CallFunction|Setswapped)
      (CallFunction|SetCurentLocation)
      (for _index (range 0 (- (Utilities|Array|Length (Variables|Default|GetallItem)) 1))
        (Variables|Default|SetIndex_0 _index)
        (for _index_2 (range (+ _index 1) (Utilities|Array|Length (Variables|Default|GetallItem)))
          (Variables|Default|SetIndex_01 _index_2)
          (Utilities|IsValid (Utilities|Array|Get(acopy) (Variables|Default|GetallItem) (Variables|Default|GetIndex_0))
            (:Is%20Valid
              (Utilities|IsValid (Utilities|Array|Get(acopy) (Variables|Default|GetallItem))
                (:Is%20Valid
                  (if (> (Math|Vector|Distance(Vector) _returnvalue (Transformation|GetActorLocation (Utilities|Array|Get(acopy) (Variables|Default|GetallItem) (Variables|Default|GetIndex_0)))) (Math|Vector|Distance(Vector) _returnvalue (Transformation|GetActorLocation (Utilities|Array|Get(acopy) (Variables|Default|GetallItem)))))
                    (Utilities|Array|Swap (Variables|Default|GetallItem) (Variables|Default|GetIndex_01) (Variables|Default|GetIndex_0))))))))))))

(event Collision|EventActorBeginOverlap
  (params (OtherActor :type Actor%20Object%20Reference)))

(event EventTick
  (params (DeltaSeconds :type Float%20%28single-precision%29))
  (CallFunction|SwapColordebug)
  (CallFunction|Debug)
  (for (_array_element _array_index) (Variables|Default|GetallItem)
    (bind _isnear (CallFunction|CheckDistancea (Transformation|GetActorLocation _array_element)))
    (if _isnear
      (bind _asbp_jalon_child (Utilities|Casting|CastToBP_JalonChild _array_element)
        (:then
          (Default|SwapColor _asbp_jalon_child)
          (Utilities|Array|RemoveIndex (Variables|Default|GetallItem) _array_index)
          (Variables|Default|Setswapped (+ (Variables|Default|Getswapped) -1))
          (Development|PrintString (Utilities|String|ToString(Integer) (Variables|Default|Getswapped)))
          (if (== (Variables|Default|Getswapped) 0)
            (Development|PrintString "gagné")))
        (:CastFailed
          (Default|SwapColor _array_element))))))

(fn ConstructionScript)

(fn SwapColordebug
  (if (Variables|Debug|Bool|Getsprintornot)
    (Variables|Color|Debug|Setcolor (Variables|Color|Debug|Getgreen))
    (else
      (Variables|Color|Debug|Setcolor (Variables|Color|Debug|Getred))))
  (if (Variables|Debug|Bool|Getforback)
    (Variables|Color|Debug|Setcolorforback (Variables|Color|Debug|Getgreen))
    (else
      (Variables|Color|Debug|Setcolorforback (Variables|Color|Debug|Getred))))
  (if (Variables|Debug|Bool|Getrightleft)
    (Variables|Color|Debug|Setcolorrightleft (Variables|Color|Debug|Getgreen))
    (else
      (Variables|Color|Debug|Setcolorrightleft (Variables|Color|Debug|Getred))))
  (if (Variables|Debug|Bool|GetyawTF)
    (Variables|Color|Debug|Setcoloryaw (Variables|Color|Debug|Getgreen))
    (else
      (Variables|Color|Debug|Setcoloryaw (Variables|Color|Debug|Getred)))))

(fn CheckDistancea
  (params (location :type Vector))
  (return (<= (Math|Vector|Distance(Vector) (Transformation|GetActorLocation) location) (Variables|Default|GetminDistance))))

(fn Debug
  (bind _returnvalue (Transformation|GetActorLocation))
  (bind _returnvalue_2 (Transformation|GetActorLocation))
  (bind _returnvalue_3 (Transformation|GetActorLocation))
  (bind _allitem (Variables|Default|GetallItem))
  (Rendering|Debug|DrawDebugSphere (Math|Vector|MakeVector (.x _returnvalue) (.y _returnvalue) (+ (.z _returnvalue) 1.2e+02)) 5.0 12 (Variables|Color|Debug|Getcolor) 0.0 5.0)
  (Rendering|Debug|DrawDebugBox (Math|Vector|MakeVector (+ (.x _returnvalue) 1e+02) (.y _returnvalue) (.z _returnvalue)) "5.000000,5.000000,5.000000" (Variables|Color|Debug|Getcolorforback) "0, 0, 0" 0.0 5.0)
  (Rendering|Debug|DrawDebugBox (Math|Vector|MakeVector (+ (.x _returnvalue) -1e+02) (.y _returnvalue) (.z _returnvalue)) "5.000000,5.000000,5.000000" (Variables|Color|Debug|Getcolorrightleft) "0, 0, 0" 0.0 5.0)
  (Rendering|Debug|DrawDebugBox (Math|Vector|MakeVector (.x _returnvalue_3) (+ (.y _returnvalue_3) 1e+02) (.z _returnvalue_3)) "5.000000,5.000000,5.000000" (Variables|Color|Debug|Getcoloryaw) "0, 0, 0" 0.0 5.0)
  (Rendering|Debug|DrawDebugBox (Math|Vector|MakeVector (.x _returnvalue_3) (+ (.y _returnvalue_3) -1e+02) (.z _returnvalue_3)) "5.000000,5.000000,5.000000" (Variables|Color|Debug|Getcoloryaw) "0, 0, 0" 0.0 5.0)
  (for _array_element _allitem
    (Default|Debug _array_element)
    (Rendering|Debug|DrawDebugLine _returnvalue_2 (Transformation|GetActorLocation _array_element) "(R=1.000000,G=0.786509,B=0.000000,A=1.000000)" 0.0 2.0)
    (bind _arrayelement (Utilities|Array|ReverseforEachLoop _allitem)
      (:Completed
        (Rendering|Debug|DrawDebugLine _returnvalue_2 (Transformation|GetActorLocation _arrayelement) "(R=1.000000,G=0.000000,B=0.000000,A=1.000000)" 0.0 2.5)))))

(fn RestartColor
  (Variables|Debug|Bool|Setsprintornot false)
  (Variables|Debug|Bool|Setforback false)
  (Variables|Debug|Bool|Setrightleft false)
  (Variables|Debug|Bool|SetyawTF false))

(fn NumbertoStart
  (for (_ _array_index) (Variables|Default|GetallItem)
    (Variables|Default|Setswapped _array_index)))

(fn Spawn
  (params (alpha :type Float%20%28double-precision%29))
  (bind _minx (Variables|Default|GetminX))
  (bind _miny (Variables|Default|GetminY))
  (bind _maxx (Variables|Default|GetmaxX))
  (bind _maxy (Variables|Default|GetmaxY))
  (bind _returnvalue (Math|Random|RandomFloatinRange _miny _maxy))
  (bind _returnvalue_2 (Math|Random|RandomFloatinRange _minx _maxx))
  (bind _returnvalue_3 (Math|Vector|MakeVector _returnvalue_2 _returnvalue 0.0))
  (bind _returnvalue_4 (Game|SpawnActorfromClass (Variables|Default|GetitemSpawn) (Math|Transform|MakeTransform (Math|Vector|MakeVector (.x _returnvalue_3) (.y _returnvalue_3) 9e+01) "0, 0, 0" "1.000000,1.000000,1.000000") "AdjustIfPossibleButDontSpawnIfColliding" "MultiplyWithRoot" 0 0))
  (Utilities|IsValid _returnvalue_4
    (:Is%20Valid
      (Utilities|Array|Add (Variables|Default|GetallItem) _returnvalue_4))))

(fn SetRandomInteger
  (Variables|Default|SetrandomInteger (Math|Random|RandomIntegerinRange 5 25)))

(fn Setswapped
  (Variables|Default|Setswapped (+ (Variables|Default|Getswapped) 1)))

(fn OnlyoneDistancedebug
  (params (location :type Vector))
  (Development|PrintString "Hello")
  (return (Utilities|Array|MakeArray (Math|Vector|Distance(Vector) (Transformation|GetActorLocation) location))))

(fn SetCurentLocation
  (Variables|Default|Setcurrentlocation (Transformation|GetActorLocation)))