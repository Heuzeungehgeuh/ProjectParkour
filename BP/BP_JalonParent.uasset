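; BP_JalonParent is a base Blueprint actor for a "jalon" (marker), with all events and the construction script empty.
; SwapColor currently just destroys the actor; its dynamic-material recolor and color comparison logic is left disconnected, as is its call in the event graph.
; Debug draws a sphere at the actor's location in DebugColor, and OnlyOne is an empty function.
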(event EventBeginPlay)

(event Collision|EventActorBeginOverlap
  (params (OtherActor :type Actor%20Object%20Reference)))

(event EventTick
  (params (DeltaSeconds :type Float%20%28single-precision%29)))

(fn ConstructionScript)

(fn SwapColor
  (Actor|DestroyActor))

(fn Debug
  (Rendering|Debug|DrawDebugSphere (Transformation|GetActorLocation) 1e+02 12 (Variables|Default|GetdebugColor) 0.0 2.0))

(fn OnlyOne)