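; Interactable item actor from a randomness exercise that, once its inherited Action activates it, spins, grows and wanders between random points.
; Each tick adds yaw, lerps scale toward a multiplied maximum through a Timeline, and draws debug shapes marking the current path.
; Movement is a timed lerp to a random XY point at fixed height, re-rolled within a distance threshold.
; The Timeline-driven rise toward Destinate is disconnected.
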(event EventBeginPlay
  (CallFunction|GetStartedLocation)
  (CallFunction|GetRandomLocation)
  (CallFunction|SetScale)
  (CallFunction|SetScaleMax)
  (CallFunction|SetDestinate))

(event Collision|EventActorBeginOverlap
  (params (OtherActor :type Actor%20Object%20Reference)))

(event EventTick
  (params (DeltaSeconds :type Float%20%28single-precision%29))
  (if (Variables|Default|GetisActivatored)
    (CallFunction|Debug)
    (CallFunction|Rotate)
    (CallFunction|MoveRandom DeltaSeconds)
    (bind _alpha (Timeline|Timeline Play)
      (:Update
        (Transformation|SetActorScale3D (Math|Vector|Lerp(Vector) (Variables|Default|Getscalestart) (Variables|Default|Getscalemax) _alpha))))))

(fn ConstructionScript
  (|CallParentFunction))

(fn Rotate
  (Transformation|SetActorRotation (Math|Rotator|MakeRotator 0.0 0.0 (+ (.yaw (Transformation|GetActorRotation)) (* (Utilities|Time|GetWorldDeltaSeconds) (Variables|Default|GetyawIncrement))))))

(fn Action
  (|CallParentFunction)
  (CallFunction|ActivateFonction))

(fn ActivateFonction
  (Variables|Default|SetisActivatored true))

(fn Elevate)

(fn Scale)

(fn GetStartedLocation
  (Variables|Default|SetstartLoc (Transformation|GetActorLocation)))

(fn GetRandomLocation
  (Variables|Default|Setdestination (Math|Vector|MakeVector (Math|Random|RandomFloatinRange (Variables|Default|GetminX) (Variables|Default|GetmaxX)) (Math|Random|RandomFloatinRange (Variables|Default|GetminY) (Variables|Default|GetmaxY)) 9e+01)))

(fn Debug
  (bind _destination (Variables|Default|Getdestination))
  (Rendering|Debug|DrawDebugSphere _destination 1e+02 12 "(R=1.000000,G=0.000000,B=0.094325,A=1.000000)" 0.0 2.0)
  (Rendering|Debug|DrawDebugLine (Variables|Default|GetstartLoc) _destination "(R=0.090634,G=0.049568,B=1.000000,A=1.000000)" 0.0 2.0))

(fn MoveRandom
  (params (delta :type Float%20%28double-precision%29))
  (bind _reacthed (CallFunction|Checktargetreach))
  (if _reacthed
    (CallFunction|ResetTime)
    (CallFunction|GetRandomLocation)
    (CallFunction|GetStartedLocation)
    (else
      (bind _alpha (CallFunction|LerpProgress (Variables|Default|GetCurrentime) (Variables|Default|GetMaxtime) delta))
      (Transformation|SetActorLocation (Math|Vector|Lerp(Vector) (Variables|Default|GetstartLoc) (Variables|Default|Getdestination) _alpha) false false))))

(fn Checktargetreach
  (return (<= (Math|Vector|Distance(Vector) (Transformation|GetActorLocation) (Variables|Default|Getdestination)) (Variables|Default|Getmindistallowed))))

(fn ResetTime
  (Variables|Default|SetCurrentime 0.0))

(fn LerpProgress
  (params (currentime :type Float%20%28double-precision%29) (maxtime :type Float%20%28double-precision%29) (delta :type Float%20%28double-precision%29))
  (if (< currentime (Variables|Default|GetMaxtime))
    (bind _output_get (Variables|Default|SetCurrentime (+ currentime delta)))
    (return (/ _output_get maxtime))
    (else
      (return (/ _output_get maxtime)))))

(fn SetScale
  (Variables|Default|Setscalestart (Transformation|GetActorScale3D)))

(fn SetScaleMax
  (Variables|Default|Setscalemax (* (Variables|Default|Getscalestart) (Variables|Default|GetscaleX10))))

(fn SetDestinate
  (Variables|Default|Setdestinate (+ (Transformation|GetActorLocation) (Variables|Default|GetupValue))))

(fn GetsIsActivate
  (return (|CallParentFunction)))