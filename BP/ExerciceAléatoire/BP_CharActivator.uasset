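; Player character that activates every item of a chosen class by walking near it, printing a win message once all are active.
; Enhanced Input drives movement, yaw rotation, and sprint and crouch, which only change walk speed.
; BeginPlay caches the items, then Tick polls each inactive one with a distance check instead of overlaps and calls its Action when in range.
; Each Tick also draws debug shapes around character and items.
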(event Input|EnhancedActionEvents|EnhancedInputActionia_Forward
  (params (ActionValue :type Float%20%28double-precision%29) (ElapsedSeconds :type Float%20%28double-precision%29) (TriggeredSeconds :type Float%20%28double-precision%29) (InputAction :type Input%20Action%20Object%20Reference :default "/Game/INPUT/ia_Forward.ia_Forward"))
  (:Triggered
    (Pawn|Input|AddMovementInput (Transformation|GetActorForwardVector) ActionValue false)))

(event Input|EnhancedActionEvents|EnhancedInputActionia_Right
  (params (ActionValue :type Float%20%28double-precision%29) (ElapsedSeconds :type Float%20%28double-precision%29) (TriggeredSeconds :type Float%20%28double-precision%29) (InputAction :type Input%20Action%20Object%20Reference :default "/Game/INPUT/ia_Right.ia_Right"))
  (:Triggered
    (Pawn|Input|AddMovementInput (Transformation|GetActorRightVector) ActionValue false)))

(event Input|EnhancedActionEvents|EnhancedInputActionia_Rotate
  (params (ActionValue :type Float%20%28double-precision%29) (ElapsedSeconds :type Float%20%28double-precision%29) (TriggeredSeconds :type Float%20%28double-precision%29) (InputAction :type Input%20Action%20Object%20Reference :default "/Game/INPUT/ia_Rotate.ia_Rotate"))
  (:Triggered
    (Pawn|Input|AddControllerYawInput ActionValue)))

(event Input|EnhancedActionEvents|EnhancedInputActionia_Sprint
  (params (ActionValue :type Boolean) (ElapsedSeconds :type Float%20%28double-precision%29) (TriggeredSeconds :type Float%20%28double-precision%29) (InputAction :type Input%20Action%20Object%20Reference :default "/Game/INPUT/ia_Sprint.ia_Sprint"))
  (bind _charactermovement (Variables|Character|GetCharacterMovement))
  (:Triggered
    (Variables|/Script/Engine.CharacterMovementComponent|SetMaxWalkSpeed _charactermovement (Variables|Default|GetsprintSpeedMax)))
  (:Completed
    (Variables|/Script/Engine.CharacterMovementComponent|SetMaxWalkSpeed _charactermovement (Variables|Default|Getspeedvaluebase))))

(event Input|EnhancedActionEvents|EnhancedInputActionia_crouch
  (params (ActionValue :type Boolean) (ElapsedSeconds :type Float%20%28double-precision%29) (TriggeredSeconds :type Float%20%28double-precision%29) (InputAction :type Input%20Action%20Object%20Reference :default "/Game/INPUT/ia_crouch.ia_crouch"))
  (bind _charactermovement (Variables|Character|GetCharacterMovement))
  (:Started
    (Variables|/Script/Engine.CharacterMovementComponent|SetMaxWalkSpeed _charactermovement (Variables|Default|GetcrouchSpeedMin)))
  (:Completed
    (Variables|/Script/Engine.CharacterMovementComponent|SetMaxWalkSpeed _charactermovement (Variables|Default|Getspeedvaluebase))))

(event EventBeginPlay
  (Input|AddMappingContext (PlayerController|LocalPlayerSubsystems|GetEnhancedInputLocalPlayerSubsystem (Game|GetPlayerController 0)) (Variables|Default|GetMapping%20Context) 0 "(bIgnoreAllPressedKeysUntilRelease=True,bForceImmediately=False)")
  (bind _outactors (Actor|GetAllActorsOfClass (Variables|Default|Gettypetofind)))
  (Variables|Default|SetAll%20Item _outactors))

(event Collision|EventActorBeginOverlap
  (params (OtherActor :type Actor%20Object%20Reference)))

(event EventTick
  (params (DeltaSeconds :type Float%20%28single-precision%29))
  (Variables|Default|SethasWon true)
  (CallFunction|Debug)
  (for _array_element (Variables|Default|GetAll%20Item)
    (if (not (Default|GetsIsActivate _array_element))
      (Variables|Default|SethasWon false)
      (bind _isnear (CallFunction|CheckDistance (Transformation|GetActorLocation _array_element)))
      (if _isnear
        (Default|Action _array_element))))
  (if (Variables|Default|GethasWon)
    (Development|PrintString "You Win")))

(fn ConstructionScript)

(fn Debug
  (bind _returnvalue (Transformation|GetActorLocation))
  (Class|KismetSystemLibrary|DrawDebugCylinder _returnvalue _returnvalue 75.0 12 "(R=1.000000,G=0.733100,B=0.000000,A=1.000000)" 0.0 2.0)
  (for _array_element (Variables|Default|GetAll%20Item)
    (Rendering|Debug|DrawDebugLine :LineStart _returnvalue :LineEnd (Transformation|GetActorLocation _array_element))
    (Rendering|Debug|DrawDebugBox (Transformation|GetActorLocation _array_element) "100.000000,100.000000,100.000000" (Variables|/Game/BP/ExerciceAléatoire/BP_ParentItem.BP_ParentItem_C|GetdebugColor _array_element) "0, 0, 0" 0.0 2.0)))

(fn CheckDistance
  (params (Location :type Vector))
  (return (<= (Math|Vector|Distance(Vector) (Transformation|GetActorLocation) Location) (Variables|Default|GetminDistance))))