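; BP_ParentItem is a base item Blueprint whose action recolors its static mesh and flags it as activated.
; Action calls SwapColor, which creates a dynamic material instance and applies MeshColor to a named vector parameter, then ActivateFonction.
; Both functions set IsActivate, which a getter exposes, while the event graph and construction script do nothing.
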(event EventBeginPlay)

(event Collision|EventActorBeginOverlap
  (params (OtherActor :type Actor%20Object%20Reference)))

(event EventTick
  (params (DeltaSeconds :type Float%20%28single-precision%29)))

(fn ConstructionScript)

(fn SwapColor
  (bind _returnvalue (Rendering|Material|CreateDynamicMaterialInstance (Variables|Default|GetStaticMesh) 0 0 "None" :!class /Script/Engine.PrimitiveComponent))
  (Rendering|Material|SetVectorParameterValue _returnvalue (Variables|Default|GetParameter%20Name) (Variables|Default|GetmeshColor) :!class /Script/Engine.MaterialInstanceDynamic)
  (Variables|Default|SetisActivate true))

(fn Action
  (CallFunction|SwapColor)
  (CallFunction|ActivateFonction))

(fn ActivateFonction
  (Variables|Default|SetisActivate true))

(fn GetsIsActivate
  (return (Variables|Default|GetisActivate)))