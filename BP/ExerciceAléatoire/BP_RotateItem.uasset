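; BP_RotateItem is an item actor that spins around its yaw axis once its action is triggered.
; Action calls the parent implementation, then ActivateFonction sets IsRotate, which nothing in this Blueprint clears.
; While that flag is set, Tick calls Rotate, which advances yaw by YawIncrement scaled by delta time for frame-rate-independent motion.
; The activation-state query simply defers to the parent class.
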(event EventBeginPlay)

(event Collision|EventActorBeginOverlap
  (params (OtherActor :type Actor%20Object%20Reference)))

(event EventTick
  (params (DeltaSeconds :type Float%20%28single-precision%29))
  (if (Variables|Default|GetIsRotate)
    (CallFunction|Rotate)))

(fn ConstructionScript
  (|CallParentFunction))

(fn Rotate
  (Transformation|SetActorRotation (Math|Rotator|MakeRotator 0.0 0.0 (+ (.yaw (Transformation|GetActorRotation)) (* (Utilities|Time|GetWorldDeltaSeconds) (Variables|Default|GetyawIncrement))))))

(fn Action
  (|CallParentFunction)
  (CallFunction|ActivateFonction))

(fn ActivateFonction
  (Variables|Default|SetIsRotate true))

(fn GetsIsActivate
  (return (|CallParentFunction)))