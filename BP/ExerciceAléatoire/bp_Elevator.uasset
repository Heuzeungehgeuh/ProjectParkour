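; Elevator actor that rises from its placed location to an offset destination when its Action is triggered.
; BeginPlay stores the start location and computes the destination by adding UpValue to it.
; Action calls the parent version, then sets IsElevate, which makes Tick play a Timeline that lerps the actor between the two points without sweep.
; IsElevate is never cleared here, so Tick keeps calling Play after activation.
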(event EventBeginPlay
  (CallFunction|StartLocation)
  (CallFunction|SetDestinate))

(event Collision|EventActorBeginOverlap
  (params (OtherActor :type Actor%20Object%20Reference)))

(event EventTick
  (params (DeltaSeconds :type Float%20%28single-precision%29))
  (if (Variables|Default|GetisElevate)
    (bind _alpha (Timeline|Timeline Play)
      (:Update
        (Transformation|SetActorLocation (Math|Vector|Lerp(Vector) (Variables|Default|Getcurrentloca) (Variables|Default|Getdestinate) _alpha) false false)))))

(fn ConstructionScript
  (|CallParentFunction))

(fn Action
  (|CallParentFunction)
  (CallFunction|ActivateFonction))

(fn ActivateFonction
  (Variables|Default|SetisElevate true))

(fn StartLocation
  (Variables|Default|Setcurrentloca (Transformation|GetActorLocation)))

(fn SetDestinate
  (Variables|Default|Setdestinate (+ (Transformation|GetActorLocation) (Variables|Default|GetupValue))))

(fn GetsIsActivate
  (return (|CallParentFunction)))