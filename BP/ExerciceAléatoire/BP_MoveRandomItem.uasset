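; An item actor that, once its Action is triggered, wanders endlessly between random points within X/Y bounds at a fixed height.
; Each Tick lerps its location from the start point to the destination over Maxtime, drawing a debug sphere and line for the current leg.
; Within the allowed distance of the target, it resets the timer, picks a new destination and restarts from its current location.
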(event EventBeginPlay
  (CallFunction|GetStartedLocation)
  (CallFunction|GetRandomLocation))

(event Collision|EventActorBeginOverlap
  (params (OtherActor :type Actor%20Object%20Reference)))

(event EventTick
  (params (DeltaSeconds :type Float%20%28single-precision%29))
  (if (Variables|Default|GetIsMoving)
    (CallFunction|Debug)
    (CallFunction|MoveRandom DeltaSeconds)))

(fn ConstructionScript
  (|CallParentFunction))

(fn GetRandomLocation
  (Variables|Default|Setdestination (Math|Vector|MakeVector (Math|Random|RandomFloatinRange (Variables|Default|GetminX) (Variables|Default|GetmaxX)) (Math|Random|RandomFloatinRange (Variables|Default|GetminY) (Variables|Default|GetmaxY)) 9e+01)))

(fn GetStartedLocation
  (Variables|Default|SetstartLoc (Transformation|GetActorLocation)))

(fn Debug
  (bind _destination (Variables|Default|Getdestination))
  (Rendering|Debug|DrawDebugSphere _destination 1e+02 12 "(R=1.000000,G=0.000000,B=0.094325,A=1.000000)" 0.0 2.0)
  (Rendering|Debug|DrawDebugLine (Variables|Default|GetstartLoc) _destination "(R=0.090634,G=0.049568,B=1.000000,A=1.000000)" 0.0 0.0))

(fn Action
  (|CallParentFunction)
  (CallFunction|ActivateFonction))

(fn ActivateFonction
  (Variables|Default|SetIsMoving true))

(fn Checktargetreach
  (return (<= (Math|Vector|Distance(Vector) (Transformation|GetActorLocation) (Variables|Default|Getdestination)) (Variables|Default|Getmindistallowed))))

(fn ResetTime
  (Variables|Default|SetCurrentime 0.0))

(fn LerpProgress
  (params (currentime :type Float%20%28double-precision%29) (maxtime :type Float%20%28double-precision%29) (delta :type Float%20%28double-precision%29))
  (if (< currentime (Variables|Default|GetMaxtime))
    (bind _output_get (Variables|Default|SetCurrentime (+ currentime delta)))
    (return (/ _output_get maxtime))
    (else
      (return (/ _output_get maxtime)))))

(fn MoveRandom
  (params (delta :type Float%20%28double-precision%29))
  (bind _reacthed (CallFunction|Checktargetreach))
  (if _reacthed
    (CallFunction|ResetTime)
    (CallFunction|GetRandomLocation)
    (CallFunction|GetStartedLocation)
    (else
      (bind _alpha (CallFunction|LerpProgress (Variables|Default|GetCurrentime) (Variables|Default|GetMaxtime) delta))
      (Transformation|SetActorLocation (Math|Vector|Lerp(Vector) (Variables|Default|GetstartLoc) (Variables|Default|Getdestination) _alpha) false false))))

(fn GetsIsActivate
  (return (|CallParentFunction)))