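; Actor Blueprint for an item that scales up smoothly once its inherited Action is triggered.
; BeginPlay stores the actor's starting scale and derives the maximum by multiplying it by ScaleX10.
; Action calls the parent, then sets IsScalling, which this Blueprint never clears.
; While that flag is set, Tick calls Play on a Timeline every frame, whose Alpha lerps the actor's scale from start to maximum.
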(event EventBeginPlay
  (CallFunction|SetScale)
  (CallFunction|SetScaleMax))

(event Collision|EventActorBeginOverlap
  (params (OtherActor :type Actor%20Object%20Reference)))

(event EventTick
  (params (DeltaSeconds :type Float%20%28single-precision%29))
  (if (Variables|Default|GetisScalling)
    (bind _alpha (Timeline|Timeline Play)
      (:Update
        (Transformation|SetActorScale3D (Math|Vector|Lerp(Vector) (Variables|Default|Getscalestart) (Variables|Default|Getscalemax) _alpha))))))

(fn ConstructionScript
  (|CallParentFunction))

(fn Action
  (|CallParentFunction)
  (CallFunction|ActivateFonction))

(fn ActivateFonction
  (Variables|Default|SetisScalling true))

(fn SetScale
  (Variables|Default|Setscalestart (Transformation|GetActorScale3D)))

(fn SetScaleMax
  (Variables|Default|Setscalemax (* (Variables|Default|Getscalestart) (Variables|Default|GetscaleX10))))

(fn GetsIsActivate
  (return (|CallParentFunction)))