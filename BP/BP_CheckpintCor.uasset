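; BP_CheckpintCor is a checkpoint actor that stores whether it has been activated.
; ActivateCheckPoint sets the activated flag, with getters exposing that flag, a debug color and a use-debug setting.
; Every tick it draws a debug sphere above the actor, green when activated and red otherwise, without consulting either debug setting.
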(event EventBeginPlay)

(event Collision|EventActorBeginOverlap
  (params (OtherActor :type Actor%20Object%20Reference)))

(event EventTick
  (params (DeltaSeconds :type Float%20%28single-precision%29))
  (CallFunction|Debug))

(fn ConstructionScript)

(fn ActivateCheckPoint
  (Variables|Default|SetisActivated true))

(fn GetDebugColor
  (return (Variables|Default|GetdebugColor)))

(fn GetUseDebug
  (return (Variables|Default|GetuseDebug)))

(fn Debug
  (bind _returnvalue (Transformation|GetActorLocation))
  (bind _returnvalue_2 (+ _returnvalue "0.000000,0.000000,100.000000"))
  (if (Variables|Default|GetisActivated)
    (Rendering|Debug|DrawDebugSphere _returnvalue_2 2e+01 12 "(R=0.193532,G=1.000000,B=0.267965,A=1.000000)" 0.0 2.0)
    (else
      (Rendering|Debug|DrawDebugSphere _returnvalue_2 2e+01 12 "(R=1.000000,G=0.172113,B=0.112380,A=1.000000)" 0.0 2.0))))

(fn GetIsActivated
  (return (Variables|Default|GetisActivated)))