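; Player character for a parkour checkpoint game, printing "Win" once all checkpoint actors are activated.
; Enhanced Input drives movement, yaw and mutually exclusive sprint and crouch toggles that only change walk speed; the combined-axis action also stores speed values, apparently for animation.
; Tick loops over actors gathered at BeginPlay, activating those within a minimum distance by distance check rather than overlap, and draws debug shapes.
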(event Input|EnhancedActionEvents|EnhancedInputActionia_Forward
  (params (ActionValue :type Float%20%28double-precision%29) (ElapsedSeconds :type Float%20%28double-precision%29) (TriggeredSeconds :type Float%20%28double-precision%29) (InputAction :type Input%20Action%20Object%20Reference :default "/Game/INPUT/ia_Forward.ia_Forward"))
  (:Triggered
    (Pawn|Input|AddMovementInput (Transformation|GetActorForwardVector) ActionValue false)))

(event Input|EnhancedActionEvents|EnhancedInputActionia_Right
  (params (ActionValue :type Float%20%28double-precision%29) (ElapsedSeconds :type Float%20%28double-precision%29) (TriggeredSeconds :type Float%20%28double-precision%29) (InputAction :type Input%20Action%20Object%20Reference :default "/Game/INPUT/ia_Right.ia_Right"))
  (:Triggered
    (Pawn|Input|AddMovementInput (Transformation|GetActorRightVector) ActionValue false)))

(event Input|EnhancedActionEvents|EnhancedInputActionia_Rotate
  (params (ActionValue :type Float%20%28double-precision%29) (ElapsedSeconds :type Float%20%28double-precision%29) (TriggeredSeconds :type Float%20%28double-precision%29) (InputAction :type Input%20Action%20Object%20Reference :default "/Game/INPUT/ia_Rotate.ia_Rotate"))
  (:Triggered
    (Pawn|Input|AddControllerYawInput ActionValue)))

(event Input|EnhancedActionEvents|EnhancedInputActionia_Sprint
  (params (ActionValue :type Boolean) (ElapsedSeconds :type Float%20%28double-precision%29) (TriggeredSeconds :type Float%20%28double-precision%29) (InputAction :type Input%20Action%20Object%20Reference :default "/Game/INPUT/ia_Sprint.ia_Sprint"))
  (:Triggered
    (CallFunction|SetisSprinting)
    (if (Variables|Default|GetisSprinting)
      (CallFunction|SetWalkSpeed (Variables|Default|GetsprintSpeed))
      (else
        (CallFunction|SetWalkSpeed (Variables|Default|GetoriginalSpeed))))))

(event Input|EnhancedActionEvents|EnhancedInputActionia_crouch
  (params (ActionValue :type Boolean) (ElapsedSeconds :type Float%20%28double-precision%29) (TriggeredSeconds :type Float%20%28double-precision%29) (InputAction :type Input%20Action%20Object%20Reference :default "/Game/INPUT/ia_crouch.ia_crouch"))
  (:Triggered
    (CallFunction|SetisCrouching)
    (if (Variables|Default|GetisCrouching)
      (CallFunction|SetWalkSpeed (Variables|Default|GetcrouchSpeedValue))
      (else
        (CallFunction|SetWalkSpeed (Variables|Default|GetoriginalSpeed))))))

(event Input|EnhancedActionEvents|EnhancedInputActionia_Entre
  (params (ActionValue :type Boolean) (ElapsedSeconds :type Float%20%28double-precision%29) (TriggeredSeconds :type Float%20%28double-precision%29) (InputAction :type Input%20Action%20Object%20Reference :default "/Game/INPUT/ia_Entre.ia_Entre")))

(event Input|EnhancedActionEvents|EnhancedInputActionia_fwd_rgtCOR
  (params (ActionValue :type Vector%202D%20Structure) (ElapsedSeconds :type Float%20%28double-precision%29) (TriggeredSeconds :type Float%20%28double-precision%29) (InputAction :type Input%20Action%20Object%20Reference :default "/Game/INPUT/ia_fwd_rgtCOR.ia_fwd_rgtCOR"))
  (:Triggered
    (Variables|Default|SetspeedAnimefwd (.x ActionValue) :!label _label)
    (Variables|Default|SetspeedAnimeRgt (.y ActionValue))
    (Pawn|Input|AddMovementInput (Transformation|GetActorForwardVector) (.x ActionValue) false)
    (Pawn|Input|AddMovementInput (Transformation|GetActorRightVector) (.y ActionValue) false))
  (:Completed
    (goto _label)))

(event EventBeginPlay
  (Input|AddMappingContext (PlayerController|LocalPlayerSubsystems|GetEnhancedInputLocalPlayerSubsystem (Game|GetPlayerController 0)) (Variables|Default|GetMapping%20Context) 0 "(bIgnoreAllPressedKeysUntilRelease=True,bForceImmediately=False)")
  (bind _outactors (Actor|GetAllActorsOfClass (Variables|Default|GettypeToFind)))
  (Variables|Default|SetallActor _outactors)
  (Variables|Default|SetoriginalSpeed (Variables|/Script/Engine.CharacterMovementComponent|GetMaxWalkSpeed (Variables|Character|GetCharacterMovement))))

(event Collision|EventActorBeginOverlap
  (params (OtherActor :type Actor%20Object%20Reference)))

(event EventTick
  (params (DeltaSeconds :type Float%20%28single-precision%29))
  (Variables|Default|SetcurrentspeedValue (Variables|/Script/Engine.CharacterMovementComponent|GetMaxWalkSpeed (Variables|Character|GetCharacterMovement)))
  (Variables|Default|SethasWon true)
  (CallFunction|Debug)
  (for _array_element (Variables|Default|GetallActor)
    (if (not (Default|GetIsActivated _array_element))
      (Variables|Default|SethasWon false)
      (bind _isnear (CallFunction|CheckDistance (Transformation|GetActorLocation _array_element)))
      (if _isnear
        (Default|ActivateCheckPoint _array_element))))
  (if (Variables|Default|GethasWon)
    (Development|PrintString "Win")))

(fn ConstructionScript)

(fn Debug
  (Rendering|Debug|DrawDebugSphere (Transformation|GetActorLocation) 1e+02 12 (Variables|Default|GetdebugColor) 0.0)
  (for _array_element (Variables|Default|GetallActor)
    (if (Default|GetUseDebug _array_element)
      (Rendering|Debug|DrawDebugBox (Transformation|GetActorLocation _array_element) "100.000000,100.000000,100.000000" (Default|GetDebugColor _array_element) "0, 0, 0" 0.0 0.0)
      (Rendering|Debug|DrawDebugLine (Transformation|GetActorLocation) (Transformation|GetActorLocation _array_element) "(R=1.000000,G=0.074743,B=0.000000,A=1.000000)" 0.0 0.0))))

(fn CheckDistance
  (params (Location :type Vector))
  (return (<= (Math|Vector|Distance(Vector) (Transformation|GetActorLocation) Location) (Variables|Default|GetminDistance))))

(fn CheckVictory
  (for _array_element (Variables|Default|GetallActor)
    (if (not (Default|GetIsActivated _array_element))
      (Variables|Default|SethasWon false))))

(fn SetisSprinting
  (bind _output_get (Variables|Default|SetisSprinting (not (Variables|Default|GetisSprinting))))
  (if (and _output_get (Variables|Default|GetisCrouching))
    (Variables|Default|SetisCrouching false)))

(fn SetisCrouching
  (bind _output_get (Variables|Default|SetisCrouching (not (Variables|Default|GetisCrouching))))
  (if (and _output_get (Variables|Default|GetisSprinting))
    (Variables|Default|SetisSprinting false)))

(fn SetWalkSpeed
  (params (value :type Float%20%28double-precision%29))
  (Variables|/Script/Engine.CharacterMovementComponent|SetMaxWalkSpeed (Variables|Character|GetCharacterMovement) value))